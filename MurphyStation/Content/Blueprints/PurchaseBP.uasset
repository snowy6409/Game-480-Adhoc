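; PurchaseBP is a base Blueprint for a one-time purchase that a player buys by interacting with it.
; Interact checks the player's Money against Cost and the CanInteract flag, then deducts the cost, locks further interaction, disables Box collision and increments the player's Purchases count.
; It then calls MakePurchase, an empty function that serves as the hook for the purchase's effect.
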(event `self.Interact`
  (params (Player :type "/Game/TopDownBP/Blueprints/TopDownCharacter Object Reference"))
  (bind _money (`/Game/TopDownBP/Blueprints/TopDownCharacter.Money` Player))
  (bind _cost (`self.Cost`))
  (if (and (>= _money _cost) (`self.Can Interact`))
    (set `/Game/TopDownBP/Blueprints/TopDownCharacter.Money` (- _money _cost) Player)
    (set `self.Can Interact` false)
    (`PrimitiveComponent.SetCollisionEnabled` (`self.Box`) "NoCollision")
    (set `/Game/TopDownBP/Blueprints/TopDownCharacter.Purchases` (+ (`/Game/TopDownBP/Blueprints/TopDownCharacter.Purchases` Player) 1) Player)
    (`self.Make Purchase` Player)))

(fn `Make Purchase`
  (params (Player :type "/Game/TopDownBP/Blueprints/TopDownCharacter Object Reference")))

(fn `UserConstructionScript`
  (`parent.UserConstructionScript`))