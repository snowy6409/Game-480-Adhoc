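; Shotgun weapon Blueprint whose Fire event shoots a horizontal fan of five FirstPersonProjectile pellets.
; Each pellet spawns at the bullet transform's location with evenly stepped yaw and zeroed pitch and roll, receiving the player and modifier-scaled damage.
; It then plays the fire sound, followed by a reload sound after half the fire-rate-adjusted delay, both at the game settings' master volume.
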(event `self.Fire`
  (params (`Bullet Transform` :type "Transform Structure") (`Damage Modifier` :type Integer) (Player :type "/Game/TopDownBP/Blueprints/TopDownCharacter Object Reference"))
  (bind _returnvalue (`self.K2_GetActorLocation`))
  (for _index (range -2 3)
    (bind _returnvalue_2 (`|SpawnActorFromClass` "/Game/FirstPersonBP/Blueprints/FirstPersonProjectile.FirstPersonProjectile_C" (`KismetMathLibrary.MakeTransform` (.location `Bullet Transform`) (`KismetMathLibrary.MakeRotator` 0.0 0.0 (+ (.yaw (.rotation `Bullet Transform`)) (* _index 3.5))) (.scale `Bullet Transform`)) "Undefined" "OverrideRootScale" null null))
    (set `/Game/FirstPersonBP/Blueprints/FirstPersonProjectile.Player` Player _returnvalue_2)
    (set `/Game/FirstPersonBP/Blueprints/FirstPersonProjectile.Damage` (+ (`self.Base Damage`) (* `Damage Modifier` (`self.Damage Scaling`))) _returnvalue_2))
  (bind _ascurrent_game_settings (cast `/Game/CurrentGameSettings` (`GameplayStatics.GetGameInstance`)))
  (bind _mastervolume (`/Game/CurrentGameSettings.MasterVolume` _ascurrent_game_settings))
  (`GameplayStatics.PlaySoundAtLocation` (`self.Fire Sound`) _returnvalue (struct) _mastervolume 1.0 0.0 null null null)
  (`KismetSystemLibrary.Delay` (/ (/ (`self.Fire Delay`) (+ (* (`/Game/TopDownBP/Blueprints/TopDownCharacter.Fire Rate Modifier` Player) 0.1) 1.0)) 2.0))
  (`GameplayStatics.PlaySoundAtLocation` "/Game/SciFiWeapLight/Sound/Shotgun/Shotgun_ReloadMag_Cue.Shotgun_ReloadMag_Cue" _returnvalue (struct) _mastervolume 1.0 0.0 null null null))

(fn `UserConstructionScript`
  (`parent.UserConstructionScript`))