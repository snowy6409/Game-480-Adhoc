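; Purchasable locker actor that dispenses a random player upgrade, priced by the current level.
; BeginPlay reads the level from the CurrentGameSettings game instance, computes a cost that grows quadratically, and builds the "Press E to Open" prompt text.
; MakePurchase turns the cube red, spawns one of six upgrade pickups at the arrow and launches it with a directional impulse using the locker's rotation.
; Payment is not handled in this graph.
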(event `self.ReceiveBeginPlay`
  (bind _ascurrent_game_settings (cast `/Game/CurrentGameSettings` (`GameplayStatics.GetGameInstance`)))
  (bind _level (`/Game/CurrentGameSettings.Level` _ascurrent_game_settings))
  (bind _returnvalue (- _level 1))
  (bind _output_get (set `self.Cost` (+ (* (* _returnvalue _returnvalue) 10) (* _level 25))))
  (set `self.Display Text` (`KismetTextLibrary.Conv_StringToText` (`KismetStringLibrary.Concat_StrStr` "Press E to Open [$" (`KismetStringLibrary.Conv_IntToString` _output_get) "]"))))

(event `self.Make Purchase`
  (params (Player :type "/Game/TopDownBP/Blueprints/TopDownCharacter Object Reference"))
  (bind _returnvalue (`self.K2_GetActorRotation`))
  (bind _returnvalue_2 (`KismetMathLibrary.MakeTransform` (`SceneComponent.K2_GetComponentLocation` (`self.Arrow`))))
  (`PrimitiveComponent.SetMaterial` (`self.Cube`) 0 "/Game/RandomJunk/Textures/Materials/ERed.ERed")
  (switch `int` (`KismetMathLibrary.RandomIntegerInRange` 0 5)
    (:`0`
      (bind _returnvalue_3 (`|SpawnActorFromClass` "/Game/Blueprints/DamageUpgrade.DamageUpgrade_C" _returnvalue_2 "AlwaysSpawn" "OverrideRootScale" null null))
      (`/Game/Blueprints/ItemBP.Directional Impulse` _returnvalue_3 _returnvalue))
    (:`1`
      (bind _returnvalue_4 (`|SpawnActorFromClass` "/Game/Blueprints/HealthUpgrade.HealthUpgrade_C" _returnvalue_2 "AlwaysSpawn" "OverrideRootScale" null null))
      (`/Game/Blueprints/ItemBP.Directional Impulse` _returnvalue_4 _returnvalue))
    (:`2`
      (bind _returnvalue_5 (`|SpawnActorFromClass` "/Game/Blueprints/OxygenUpgrade.OxygenUpgrade_C" _returnvalue_2 "AlwaysSpawn" "OverrideRootScale" null null))
      (`/Game/Blueprints/ItemBP.Directional Impulse` _returnvalue_5 _returnvalue))
    (:`3`
      (bind _returnvalue_6 (`|SpawnActorFromClass` "/Game/Blueprints/FireRateUpgrade.FireRateUpgrade_C" _returnvalue_2 "AlwaysSpawn" "OverrideRootScale" null null))
      (`/Game/Blueprints/ItemBP.Directional Impulse` _returnvalue_6 _returnvalue))
    (:`4`
      (bind _returnvalue_7 (`|SpawnActorFromClass` "/Game/Blueprints/ReloadUpgrade.ReloadUpgrade_C" _returnvalue_2 "AlwaysSpawn" "OverrideRootScale" null null))
      (`/Game/Blueprints/ItemBP.Directional Impulse` _returnvalue_7 _returnvalue))
    (:`5`
      (bind _returnvalue_8 (`|SpawnActorFromClass` "/Game/Blueprints/SpeedUpgrade.SpeedUpgrade_C" _returnvalue_2 "AlwaysSpawn" "OverrideRootScale" null null))
      (`/Game/Blueprints/ItemBP.Directional Impulse` _returnvalue_8 _returnvalue))))

(fn `UserConstructionScript`
  (`parent.UserConstructionScript`))