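; ItemBP is an item Blueprint that spins in the world and can be tossed with physics impulses.
; Tick adds a fixed yaw step to the Root component each frame, so spin speed depends on frame rate.
; Directional Impulse launches Root along a given rotation's horizontal forward with randomized spread, strength and upward lift.
; Random Impulse gives Root a smaller random horizontal push with similar upward lift.
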(event `self.ReceiveTick`
  (params (DeltaSeconds :type "Float (single-precision)"))
  (bind _root (`self.Root`))
  (`SceneComponent.K2_SetWorldRotation` _root (`KismetMathLibrary.MakeRotator` (.roll (`SceneComponent.K2_GetComponentRotation` _root)) (.pitch (`SceneComponent.K2_GetComponentRotation` _root)) (+ (.yaw (`SceneComponent.K2_GetComponentRotation` _root)) 1.0)) false false))

(fn `Directional Impulse`
  (params (Direction :type "Rotator Structure"))
  (`PrimitiveComponent.AddImpulse` (`self.Root`) (`KismetMathLibrary.MakeVector` (* (+ (.x (`KismetMathLibrary.GetForwardVector` Direction)) (`KismetMathLibrary.RandomFloatInRange` -0.6 0.6)) (`KismetMathLibrary.RandomFloatInRange` 200.0 400.0)) (* (+ (.y (`KismetMathLibrary.GetForwardVector` Direction)) (`KismetMathLibrary.RandomFloatInRange` -0.6 0.6)) (`KismetMathLibrary.RandomFloatInRange` 200.0 400.0)) (`KismetMathLibrary.RandomFloatInRange` 100.0 300.0)) "None" false))

(fn `Random Impulse`
  (`PrimitiveComponent.AddImpulse` (`self.Root`) (`KismetMathLibrary.MakeVector` (`KismetMathLibrary.RandomFloatInRange` -100.0 100.0) (`KismetMathLibrary.RandomFloatInRange` -100.0 100.0) (`KismetMathLibrary.RandomFloatInRange` 100.0 300.0)) "None" false))

(fn `UserConstructionScript`
  (`parent.UserConstructionScript`))