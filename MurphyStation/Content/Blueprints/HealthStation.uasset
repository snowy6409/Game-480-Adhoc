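; HealthStation is a purchasable interactable that restores player health for a price.
; On BeginPlay it reads Level from the CurrentGameSettings game instance to scale the cost and build the prompt text.
; MakePurchase adds a level-scaled heal, or a fixed amount if the game instance cast fails, clamped to the player's maximum, then turns the cube red.
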(event `self.ReceiveBeginPlay`
  (bind _ascurrent_game_settings (cast `/Game/CurrentGameSettings` (`GameplayStatics.GetGameInstance`)))
  (bind _output_get (set `self.Cost` (* (`/Game/CurrentGameSettings.Level` _ascurrent_game_settings) 15)))
  (set `self.Display Text` (`KismetTextLibrary.Conv_StringToText` (`KismetStringLibrary.Concat_StrStr` "Press E to Restore Health [$" (`KismetStringLibrary.Conv_IntToString` _output_get) "]"))))

(event `self.Make Purchase`
  (params (Player :type "/Game/TopDownBP/Blueprints/TopDownCharacter Object Reference"))
  (bind _player_max_health (`/Game/TopDownBP/Blueprints/TopDownCharacter.Player Max Health` Player))
  (bind _player_health (`/Game/TopDownBP/Blueprints/TopDownCharacter.Player Health` Player))
  (bind _ascurrent_game_settings (cast `/Game/CurrentGameSettings` (`GameplayStatics.GetGameInstance`))
    (:`then`
      (set `/Game/TopDownBP/Blueprints/TopDownCharacter.Player Health` (`KismetMathLibrary.Clamp` (+ _player_health (* (`/Game/CurrentGameSettings.Level` _ascurrent_game_settings) 10) 40) 0 _player_max_health) Player))
    (:`CastFailed`
      (set `/Game/TopDownBP/Blueprints/TopDownCharacter.Player Health` (`KismetMathLibrary.Clamp` (+ _player_health 50) 0 _player_max_health) Player)))
  (`PrimitiveComponent.SetMaterial` (`self.Cube`) 0 "/Game/RandomJunk/Textures/Materials/ERed.ERed"))

(fn `UserConstructionScript`
  (`parent.UserConstructionScript`))