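; Ammo pickup that refills the player's reserve ammo for one of several weapon types.
; SelectAmmoType usually matches the given weapon, with a small chance of a random type, and always rolls randomly when the weapon is zero.
; PickUp adds that type's amount clamped to the reserve maximum, plays a per-type sound scaled by master volume, and returns false if the reserve is already full.
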(fn `Pick Up`
  (params (Player :type "/Game/TopDownBP/Blueprints/TopDownCharacter Object Reference"))
  (returns (Used :type Boolean))
  (bind _returnvalue (`self.K2_GetActorLocation`))
  (bind _reserve_ammo (`/Game/TopDownBP/Blueprints/TopDownCharacter.Reserve Ammo` Player))
  (bind _ammo_type (`self.Ammo Type`))
  (bind _ammo_type_2 (`self.Ammo Type`))
  (bind _output (`|GetArrayItem` _reserve_ammo _ammo_type))
  (bind _output_2 (`|GetArrayItem` (`/Game/TopDownBP/Blueprints/TopDownCharacter.Max Reserve Ammo` Player) _ammo_type))
  (if (< _output _output_2)
    (`KismetArrayLibrary.Array_Set` _reserve_ammo _ammo_type_2 (`KismetMathLibrary.Clamp` (+ _output (`|GetArrayItem` (`self.Pickup Amount`) _ammo_type)) 0 _output_2))
    (bind _ascurrent_game_settings (cast `/Game/CurrentGameSettings` (`GameplayStatics.GetGameInstance`))
      (:`then`
        (switch `int` _ammo_type_2
          (:`Default`
            _)
          (:`0`
            _)
          (:`1`
            (bind _mastervolume (`/Game/CurrentGameSettings.MasterVolume` _ascurrent_game_settings))
            (`GameplayStatics.PlaySoundAtLocation` "/Game/SciFiWeapLight/Sound/SniperRifle/SR_AmmoPickup_Cue.SR_AmmoPickup_Cue" _returnvalue (struct) _mastervolume 1.0 0.0 null null null))
          (:`2`
            (`GameplayStatics.PlaySoundAtLocation` "/Game/SciFiWeapLight/Sound/Shotgun/Shotgun_AmmoPickup_Cue.Shotgun_AmmoPickup_Cue" _returnvalue (struct) _mastervolume 1.0 0.0 null null null))
          (:`3`
            (`GameplayStatics.PlaySoundAtLocation` "/Game/SciFiWeapLight/Sound/GrenadeLauncher/GL_AmmoPickup_Cue.GL_AmmoPickup_Cue" _returnvalue (struct) _mastervolume 1.0 0.0 null null null))))
      (:`CastFailed`
        _))
    (return true)
    (else
      (return false))))

(fn `Select Ammo Type`
  (params (Weapon :type Integer))
  (if (== Weapon 0)
    (set `self.Ammo Type` (`KismetMathLibrary.RandomIntegerInRange` 1 3) :!label _label)
    (elif (>= (`KismetMathLibrary.RandomIntegerInRange` 1 100) 85)
      (goto _label)
      (else
        (set `self.Ammo Type` Weapon)))))

(fn `UserConstructionScript`)