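; WeaponCrate is a purchasable crate that offers the player a random weapon for cash.
; On BeginPlay it reads the level from the CurrentGameSettings game instance, scales the cost linearly with it and builds the interaction prompt.
; MakePurchase turns the cube red, spawns a WeaponDrop at the arrow and launches it using the crate's rotation.
; Payment and weapon selection are handled outside this graph.
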(event `self.ReceiveBeginPlay`
  (bind _ascurrent_game_settings (cast `/Game/CurrentGameSettings` (`GameplayStatics.GetGameInstance`)))
  (bind _output_get (set `self.Cost` (+ (* (- (`/Game/CurrentGameSettings.Level` _ascurrent_game_settings) 1) 75) 125)))
  (set `self.Display Text` (`KismetTextLibrary.Conv_StringToText` (`KismetStringLibrary.Concat_StrStr` "Press E to for a Random Weapon [$" (`KismetStringLibrary.Conv_IntToString` _output_get) "]"))))

(event `self.Make Purchase`
  (params (Player :type "/Game/TopDownBP/Blueprints/TopDownCharacter Object Reference"))
  (`PrimitiveComponent.SetMaterial` (`self.Cube`) 0 "/Game/RandomJunk/Textures/Materials/ERed.ERed")
  (bind _returnvalue (`|SpawnActorFromClass` "/Game/Blueprints/WeaponDrop.WeaponDrop_C" (`KismetMathLibrary.MakeTransform` (`SceneComponent.K2_GetComponentLocation` (`self.Arrow`))) "Undefined" "OverrideRootScale" null null))
  (`/Game/Blueprints/ItemBP.Directional Impulse` _returnvalue (`self.K2_GetActorRotation`)))

(fn `UserConstructionScript`
  (`parent.UserConstructionScript`))