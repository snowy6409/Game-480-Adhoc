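; Health pickup that restores a small fixed amount of health to the player.
; PickUp adds health only when the player is below maximum, clamps the result to that maximum, and returns whether the pickup was used.
; A pickup sound scaled by the game settings' master volume is present but disconnected, so it never plays.
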(fn `Pick Up`
  (params (Player :type "/Game/TopDownBP/Blueprints/TopDownCharacter Object Reference"))
  (returns (Used :type Boolean))
  (bind _player_max_health (`/Game/TopDownBP/Blueprints/TopDownCharacter.Player Max Health` Player))
  (bind _player_health (`/Game/TopDownBP/Blueprints/TopDownCharacter.Player Health` Player))
  (if (< _player_health _player_max_health)
    (set `/Game/TopDownBP/Blueprints/TopDownCharacter.Player Health` (`KismetMathLibrary.Clamp` (+ _player_health 5) 0 _player_max_health) Player)
    (return true)
    (else
      (return false))))

(fn `UserConstructionScript`)