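; Interactable loot crate that opens once and ejects a random damage, health or oxygen upgrade.
; On Interact it sets Opened, disables the Box collision, spawns the chosen upgrade at the Arrow's location and launches it with DirectionalImpulse using the crate's rotation.
; ShowText and HideText pass through to the parent only while the crate is unopened.
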(event `self.Interact`
  (params (Player :type "/Game/TopDownBP/Blueprints/TopDownCharacter Object Reference"))
  (bind _returnvalue (`self.K2_GetActorRotation`))
  (bind _returnvalue_2 (`KismetMathLibrary.MakeTransform` (`SceneComponent.K2_GetComponentLocation` (`self.Arrow`))))
  (if (not (`self.Opened`))
    (set `self.Opened` true)
    (`PrimitiveComponent.SetCollisionEnabled` (`self.Box`) "NoCollision")
    (switch `int` (`KismetMathLibrary.RandomIntegerInRange` 0 2)
      (:`0`
        (bind _returnvalue_3 (`|SpawnActorFromClass` "/Game/Blueprints/DamageUpgrade.DamageUpgrade_C" _returnvalue_2 "Undefined" "OverrideRootScale" null null))
        (`/Game/Blueprints/ItemBP.Directional Impulse` _returnvalue_3 _returnvalue))
      (:`1`
        (bind _returnvalue_4 (`|SpawnActorFromClass` "/Game/Blueprints/HealthUpgrade.HealthUpgrade_C" _returnvalue_2 "Undefined" "OverrideRootScale" null null))
        (`/Game/Blueprints/ItemBP.Directional Impulse` _returnvalue_4 _returnvalue))
      (:`2`
        (bind _returnvalue_5 (`|SpawnActorFromClass` "/Game/Blueprints/OxygenUpgrade.OxygenUpgrade_C" _returnvalue_2 "Undefined" "OverrideRootScale" null null))
        (`/Game/Blueprints/ItemBP.Directional Impulse` _returnvalue_5 _returnvalue)))))

(event `self.Show Text`
  (params (Player :type "/Game/TopDownBP/Blueprints/TopDownCharacter Object Reference"))
  (if (not (`self.Opened`))
    (`parent.Show Text` Player)))

(event `self.Hide Text`
  (params (Player :type "/Game/TopDownBP/Blueprints/TopDownCharacter Object Reference"))
  (if (not (`self.Opened`))
    (`parent.Hide Text` Player)))

(fn `UserConstructionScript`
  (`parent.UserConstructionScript`))