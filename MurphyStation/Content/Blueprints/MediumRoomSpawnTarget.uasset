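; Placeholder actor that spawns a medium room (Command, Engineering, Living or Utility, with Generic as fallback) at its own transform, then destroys itself.
; On BeginPlay it picks a random type if ExternalChoice is -1; otherwise it waits for SpawnNow, which spawns the type ExternalChoice selects.
; SetDoors copies its four directional door values to the new room and calls SetWallState to update the walls.
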(event `SpawnNow`
  (bind _returnvalue (`self.GetTransform`))
  (switch `int` (`self.ExternalChoice`)
    (:`Default`
      (bind _returnvalue_2 (`|SpawnActorFromClass` "/Game/Rooms/RM_Medium_Generic.RM_Medium_Generic_C" _returnvalue "AlwaysSpawn" "OverrideRootScale" null null))
      (`self.Set Doors` _returnvalue_2))
    (:`0`
      (bind _returnvalue_3 (`|SpawnActorFromClass` "/Game/Rooms/RM_Medium_Command.RM_Medium_Command_C" _returnvalue "AlwaysSpawn" "OverrideRootScale" null null))
      (`self.Set Doors` _returnvalue_3))
    (:`1`
      (bind _returnvalue_4 (`|SpawnActorFromClass` "/Game/Rooms/RM_Medium_Engineering.RM_Medium_Engineering_C" _returnvalue "AlwaysSpawn" "OverrideRootScale" null null))
      (`self.Set Doors` _returnvalue_4))
    (:`2`
      (bind _returnvalue_5 (`|SpawnActorFromClass` "/Game/Rooms/RM_Medium_Living.RM_Medium_Living_C" _returnvalue "AlwaysSpawn" "OverrideRootScale" null null))
      (`self.Set Doors` _returnvalue_5))
    (:`3`
      (bind _returnvalue_6 (`|SpawnActorFromClass` "/Game/Rooms/RM_Medium_Utility.RM_Medium_Utility_C" _returnvalue "AlwaysSpawn" "OverrideRootScale" null null))
      (`self.Set Doors` _returnvalue_6)))
  (`self.K2_DestroyActor`))

(event `self.ReceiveBeginPlay`
  (bind _returnvalue (`self.GetTransform`))
  (if (not (!= (`self.ExternalChoice`) -1))
    (switch `int` (`KismetMathLibrary.RandomIntegerInRange` 0 3)
      (:`Default`
        (bind _returnvalue_2 (`|SpawnActorFromClass` "/Game/Rooms/RM_Medium_Generic.RM_Medium_Generic_C" _returnvalue "AlwaysSpawn" "OverrideRootScale" null null))
        (`self.Set Doors` _returnvalue_2))
      (:`0`
        (bind _returnvalue_3 (`|SpawnActorFromClass` "/Game/Rooms/RM_Medium_Command.RM_Medium_Command_C" _returnvalue "AlwaysSpawn" "OverrideRootScale" null null))
        (`self.Set Doors` _returnvalue_3))
      (:`1`
        (bind _returnvalue_4 (`|SpawnActorFromClass` "/Game/Rooms/RM_Medium_Engineering.RM_Medium_Engineering_C" _returnvalue "AlwaysSpawn" "OverrideRootScale" null null))
        (`self.Set Doors` _returnvalue_4))
      (:`2`
        (bind _returnvalue_5 (`|SpawnActorFromClass` "/Game/Rooms/RM_Medium_Living.RM_Medium_Living_C" _returnvalue "AlwaysSpawn" "OverrideRootScale" null null))
        (`self.Set Doors` _returnvalue_5))
      (:`3`
        (bind _returnvalue_6 (`|SpawnActorFromClass` "/Game/Rooms/RM_Medium_Utility.RM_Medium_Utility_C" _returnvalue "AlwaysSpawn" "OverrideRootScale" null null))
        (`self.Set Doors` _returnvalue_6)))
    (`self.K2_DestroyActor`)))

(fn `Set Doors`
  (params (Room :type "/Game/Rooms/RoomBP Object Reference (by ref)"))
  (set `/Game/Rooms/RoomBP.Up` (`self.Door Up`) Room)
  (set `/Game/Rooms/RoomBP.Down` (`self.Door Down`) Room)
  (set `/Game/Rooms/RoomBP.Left` (`self.Door Left`) Room)
  (set `/Game/Rooms/RoomBP.Right` (`self.Door Right`) Room)
  (`/Game/Rooms/RoomBP.Set Wall State` Room))

(fn `UserConstructionScript`)