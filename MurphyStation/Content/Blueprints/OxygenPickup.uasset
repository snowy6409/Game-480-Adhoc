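; Oxygen pickup that restores a fixed amount of a player's oxygen.
; PickUp adds the oxygen only when the player is below maximum, clamps the result to that maximum and returns whether anything was applied.
; A pickup sound scaled by the master volume from CurrentGameSettings is present but disconnected, so it never plays.
; The construction script only calls its parent.
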(fn `Pick Up`
  (params (Player :type "/Game/TopDownBP/Blueprints/TopDownCharacter Object Reference"))
  (returns (Used :type Boolean))
  (bind _max_oxygen (`/Game/TopDownBP/Blueprints/TopDownCharacter.Max Oxygen` Player))
  (bind _current_oxygen (`/Game/TopDownBP/Blueprints/TopDownCharacter.Current Oxygen` Player))
  (if (< _current_oxygen _max_oxygen)
    (set `/Game/TopDownBP/Blueprints/TopDownCharacter.Current Oxygen` (`KismetMathLibrary.Clamp` (+ _current_oxygen 10) 0 _max_oxygen) Player)
    (return true)
    (else
      (return false))))

(fn `UserConstructionScript`
  (`parent.UserConstructionScript`))