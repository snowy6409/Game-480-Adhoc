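; Interactable console that starts the self-destruct countdown in the top-down game.
; Entering its box enables that player's input on the console and shows a HUD prompt unless a countdown is active; leaving reverses both.
; Interact turns the hologram meshes red, turns off every RoomBP's lights if power is not restored, and calls StartCountdown on TopDownGameMode.
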(event `self.Box.OnComponentBeginOverlap`
  (params (OverlappedComponent :type "PrimitiveComponent Object Reference") (OtherActor :type "Actor Object Reference") (OtherComp :type "PrimitiveComponent Object Reference") (OtherBodyIndex :type Integer) (bFromSweep :type Boolean) (SweepResult :type "HitResult Structure (by ref)"))
  (bind _astop_down_character (cast `/Game/TopDownBP/Blueprints/TopDownCharacter` OtherActor))
  (bind _astop_down_game_mode (cast `/Game/TopDownBP/Blueprints/TopDownGameMode` (`GameplayStatics.GetGameMode`)))
  (if (not (`/Game/TopDownBP/Blueprints/TopDownGameMode.Countdown Active` _astop_down_game_mode))
    (`self.EnableInput` (`GameplayStatics.GetPlayerController` (`/Game/TopDownBP/Blueprints/TopDownCharacter.Player Index` _astop_down_character)))
    (`/Game/Widget/HUD.Set Help Text` (`/Game/TopDownBP/Blueprints/TopDownCharacter.Hudref` _astop_down_character) "Press E to Initiate Self-Destruct Sequence")))

(event `self.Box.OnComponentEndOverlap`
  (params (OverlappedComponent :type "PrimitiveComponent Object Reference") (OtherActor :type "Actor Object Reference") (OtherComp :type "PrimitiveComponent Object Reference") (OtherBodyIndex :type Integer))
  (bind _astop_down_character (cast `/Game/TopDownBP/Blueprints/TopDownCharacter` OtherActor))
  (`self.DisableInput` (`GameplayStatics.GetPlayerController` (`/Game/TopDownBP/Blueprints/TopDownCharacter.Player Index` _astop_down_character)))
  (`/Game/Widget/HUD.Set Help Text` (`/Game/TopDownBP/Blueprints/TopDownCharacter.Hudref` _astop_down_character) ""))

(event `InputAction|Interact`
  (params (Key :type "Key Structure"))
  (:`Pressed`
    (`PrimitiveComponent.SetMaterial` (`self.Sphere`) 0 "/Game/RandomJunk/Textures/Materials/HologramMat_Red.HologramMat_Red")
    (`PrimitiveComponent.SetMaterial` (`self.Cube`) 0 "/Game/RandomJunk/Textures/Materials/HologramMat2_Red.HologramMat2_Red")
    (`PrimitiveComponent.SetMaterial` (`self.Cube1`) 0 "/Game/RandomJunk/Textures/Materials/HologramMat2_Red.HologramMat2_Red")
    (`PrimitiveComponent.SetMaterial` (`self.Cube2`) 0 "/Game/RandomJunk/Textures/Materials/HologramMat2_Red.HologramMat2_Red")
    (`PrimitiveComponent.SetMaterial` (`self.Cube3`) 0 "/Game/RandomJunk/Textures/Materials/HologramMat2_Red.HologramMat2_Red")
    (bind _astop_down_game_mode (cast `/Game/TopDownBP/Blueprints/TopDownGameMode` (`GameplayStatics.GetGameMode`)))
    (if (not (`/Game/TopDownBP/Blueprints/TopDownGameMode.Power Restored` _astop_down_game_mode))
      (bind _outactors (`GameplayStatics.GetAllActorsOfClass` "/Game/Rooms/RoomBP.RoomBP_C"))
      (for _array_element _outactors
        (`/Game/Rooms/RoomBP.Turn Off Lights` _array_element)))
    (`/Game/TopDownBP/Blueprints/TopDownGameMode.Start Countdown` _astop_down_game_mode)))

(fn `UserConstructionScript`)