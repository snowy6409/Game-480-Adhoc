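; SpawnFloorArray is a Blueprint that builds a fixed floor layout of rooms and hallways at BeginPlay.
; A nested loop walks a 48x48 grid, passing every cell through hard-coded SpawnRoomWithCords calls that spawn only on a coordinate match.
; Large rooms form the center and four cardinal ends, medium rooms the diagonals, with hallways mostly along the axes.
; Grid indices scale by 302 units into X/Y locations, and spawning always succeeds, adjusting for collisions where possible.
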(event `self.ReceiveBeginPlay`
  (for _index (range 48)
    (for _index_2 (range 48)
      (`self.SpawnRoomWithCords` _index_2 _index 24 6 "/Game/Rooms/RM_Large_Generic.RM_Large_Generic_C")
      (`self.SpawnRoomWithCords` _index_2 _index 6 24 "/Game/Rooms/RM_Large_Generic.RM_Large_Generic_C")
      (`self.SpawnRoomWithCords` _index_2 _index 24 24 "/Game/Rooms/RM_Large_Generic.RM_Large_Generic_C")
      (`self.SpawnRoomWithCords` _index_2 _index 24 42 "/Game/Rooms/RM_Large_Generic.RM_Large_Generic_C")
      (`self.SpawnRoomWithCords` _index_2 _index 42 24 "/Game/Rooms/RM_Large_Generic.RM_Large_Generic_C")
      (`self.SpawnRoomWithCords` _index_2 _index 16 16 "/Game/Rooms/RM_Medium_Generic.RM_Medium_Generic_C")
      (`self.SpawnRoomWithCords` _index_2 _index 16 32 "/Game/Rooms/RM_Medium_Generic.RM_Medium_Generic_C")
      (`self.SpawnRoomWithCords` _index_2 _index 32 16 "/Game/Rooms/RM_Medium_Generic.RM_Medium_Generic_C")
      (`self.SpawnRoomWithCords` _index_2 _index 32 32 "/Game/Rooms/RM_Medium_Generic.RM_Medium_Generic_C")
      (`self.SpawnRoomWithCords` _index_2 _index 15 24 "/Game/Rooms/Hallway.Hallway_C")
      (`self.SpawnRoomWithCords` _index_2 _index 24 15 "/Game/Rooms/Hallway.Hallway_C")
      (`self.SpawnRoomWithCords` _index_2 _index 24 33 "/Game/Rooms/Hallway.Hallway_C")
      (`self.SpawnRoomWithCords` _index_2 _index 33 24 "/Game/Rooms/Hallway.Hallway_C")
      (`self.SpawnRoomWithCords` _index_2 _index 30 24 "/Game/Rooms/Hallway.Hallway_C")
      (`self.SpawnRoomWithCords` _index_2 _index 24 30 "/Game/Rooms/Hallway.Hallway_C")
      (`self.SpawnRoomWithCords` _index_2 _index 12 24 "/Game/Rooms/Hallway.Hallway_C")
      (`self.SpawnRoomWithCords` _index_2 _index 24 12 "/Game/Rooms/Hallway.Hallway_C")
      (`self.SpawnRoomWithCords` _index_2 _index 36 24 "/Game/Rooms/Hallway.Hallway_C")
      (`self.SpawnRoomWithCords` _index_2 _index 24 36 "/Game/Rooms/Hallway.Hallway_C")
      (`self.SpawnRoomWithCords` _index_2 _index 18 24 "/Game/Rooms/Hallway.Hallway_C")
      (`self.SpawnRoomWithCords` _index_2 _index 24 18 "/Game/Rooms/Hallway.Hallway_C")
      (`self.SpawnRoomWithCords` _index_2 _index 21 33 "/Game/Rooms/Hallway.Hallway_C"))))

(fn `SpawnRoomWithCords`
  (params (InputX :type Integer) (InputY :type Integer) (IndexX :type Integer) (IndexY :type Integer) (`Room Class` :type "Actor Class Reference"))
  (if (and (== InputX IndexX) (== InputY IndexY))
    (`|SpawnActorFromClass` `Room Class` (`KismetMathLibrary.MakeTransform` (`KismetMathLibrary.MakeVector` (* InputX 302.0) (* InputY 302.0))) "AdjustIfPossibleButAlwaysSpawn" "OverrideRootScale" null null)))

(fn `UserConstructionScript`)