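; Weapon pickup actor that becomes a random assault rifle, shotgun or sniper rifle on BeginPlay, setting its mesh and pickup prompt to match.
; Interact has the player equip that weapon and destroys the pickup, unless the player's secondary weapon is already the same type.
; ShowText applies the same check to show either the pickup prompt or "Already Equipped" on the player's HUD.
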(event `self.ReceiveBeginPlay`
  (bind _skeletalmesh (`self.SkeletalMesh`))
  (bind _returnvalue (`KismetTextLibrary.Conv_TextToString` (`self.Display Text`)))
  (bind _output_get (set `self.Weapon Type` (`KismetMathLibrary.RandomIntegerInRange` 1 3)))
  (set `self.Display Text` "Press E to Pick Up ")
  (switch `int` _output_get
    (:`1`
      (`SkinnedMeshComponent.SetSkinnedAssetAndUpdate` _skeletalmesh "/Game/SciFiWeapLight/Weapons/White_AssaultRifle.White_AssaultRifle" true)
      (set `self.Display Text` (`KismetTextLibrary.Conv_StringToText` (`KismetStringLibrary.Concat_StrStr` _returnvalue "Assault Rifle"))))
    (:`2`
      (`SkinnedMeshComponent.SetSkinnedAssetAndUpdate` _skeletalmesh "/Game/SciFiWeapLight/Weapons/White_Shotgun.White_Shotgun" true)
      (set `self.Display Text` (`KismetTextLibrary.Conv_StringToText` (`KismetStringLibrary.Concat_StrStr` _returnvalue "Shotgun"))))
    (:`3`
      (`SkinnedMeshComponent.SetSkinnedAssetAndUpdate` _skeletalmesh "/Game/SciFiWeapLight/Weapons/White_SniperRifle.White_SniperRifle" true)
      (set `self.Display Text` (`KismetTextLibrary.Conv_StringToText` (`KismetStringLibrary.Concat_StrStr` _returnvalue "Sniper Rifle"))))))

(event `self.Interact`
  (params (Player :type "/Game/TopDownBP/Blueprints/TopDownCharacter Object Reference"))
  (bind _weapon_type (`self.Weapon Type`))
  (bind _secondary_weapon (`/Game/TopDownBP/Blueprints/TopDownCharacter.Secondary Weapon` Player))
  (if (`KismetSystemLibrary.IsValid` _secondary_weapon)
    (if (!= _weapon_type (`/Game/Weapons/WeaponBP.Weapon Type` _secondary_weapon))
      (switch `int` _weapon_type :!label _label
        (:`1`
          (`/Game/TopDownBP/Blueprints/TopDownCharacter.Equip Weapon` Player "/Game/Weapons/AssaultRifle.AssaultRifle_C"))
        (:`2`
          (`/Game/TopDownBP/Blueprints/TopDownCharacter.Equip Weapon` Player "/Game/Weapons/Shotgun.Shotgun_C"))
        (:`3`
          (`/Game/TopDownBP/Blueprints/TopDownCharacter.Equip Weapon` Player "/Game/Weapons/SniperRifle.SniperRifle_C")))
      (`self.K2_DestroyActor`))
    (else
      (goto _label))))

(event `self.Show Text`
  (params (Player :type "/Game/TopDownBP/Blueprints/TopDownCharacter Object Reference"))
  (bind _secondary_weapon (`/Game/TopDownBP/Blueprints/TopDownCharacter.Secondary Weapon` Player))
  (bind _hudref (`/Game/TopDownBP/Blueprints/TopDownCharacter.Hudref` Player))
  (if (`KismetSystemLibrary.IsValid` _secondary_weapon)
    (if (== (`self.Weapon Type`) (`/Game/Weapons/WeaponBP.Weapon Type` _secondary_weapon))
      (`/Game/Widigit]/HUD.Set Help Text` _hudref "Already Equipped")
      (else
        (`/Game/Widigit]/HUD.Set Help Text` _hudref (`self.Display Text`) :!label _label_2)))
    (else
      (goto _label_2))))

(fn `UserConstructionScript`
  (`parent.UserConstructionScript`))