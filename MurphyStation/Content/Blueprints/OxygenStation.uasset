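; Oxygen station interactable that sells the player a one-time oxygen refill for money.
; On BeginPlay it reads the level from the CurrentGameSettings game instance to set a level-scaled cost and the prompt text showing it.
; Interact checks money and availability, deducts the cost, and adds a level-scaled amount of oxygen clamped to the player's maximum.
; It then disables itself, turning off box collision and switching the cube to a red material.
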(event `self.ReceiveBeginPlay`
  (bind _ascurrent_game_settings (cast `/Game/CurrentGameSettings` (`GameplayStatics.GetGameInstance`)))
  (bind _output_get (set `self.Cost` (* (`/Game/CurrentGameSettings.Level` _ascurrent_game_settings) 10)))
  (set `self.Display Text` (`KismetTextLibrary.Conv_StringToText` (`KismetStringLibrary.Concat_StrStr` "Press E to Restore Oxygen [$" (`KismetStringLibrary.Conv_IntToString` _output_get) "]"))))

(event `self.Interact`
  (params (Player :type "/Game/TopDownBP/Blueprints/TopDownCharacter Object Reference"))
  (bind _money (`/Game/TopDownBP/Blueprints/TopDownCharacter.Money` Player))
  (if (and (>= _money (`self.Cost`)) (`self.Can Interact`))
    (bind _ascurrent_game_settings (cast `/Game/CurrentGameSettings` (`GameplayStatics.GetGameInstance`)))
    (set `/Game/TopDownBP/Blueprints/TopDownCharacter.Money` (- _money (`self.Cost`)) Player)
    (set `/Game/TopDownBP/Blueprints/TopDownCharacter.Current Oxygen` (`KismetMathLibrary.Clamp` (+ (`/Game/TopDownBP/Blueprints/TopDownCharacter.Current Oxygen` Player) (* (`/Game/CurrentGameSettings.Level` _ascurrent_game_settings) 10) 40) 0 (`/Game/TopDownBP/Blueprints/TopDownCharacter.Max Oxygen` Player)) Player)
    (set `self.Can Interact` false)
    (`PrimitiveComponent.SetCollisionEnabled` (`self.Box`) "NoCollision")
    (`PrimitiveComponent.SetMaterial` (`self.Cube`) 0 "/Game/RandomJunk/Textures/Materials/ERed.ERed")))

(fn `UserConstructionScript`
  (`parent.UserConstructionScript`))