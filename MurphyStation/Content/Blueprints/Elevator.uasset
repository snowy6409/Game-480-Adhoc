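; Elevator exit that lets players evacuate the station once the game mode's countdown is active.
; Its Box overlap shows HUD help text and, during the countdown, enables the actor's input for that player, disabling it when they leave.
; Interact in Endless mode increments the level, saves every character and opens AlphaLayput.
; Otherwise it pauses the game, hides all characters and gives each player a GameOver escape screen with UI-only input.
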(event `self.Box.OnComponentBeginOverlap`
  (params (OverlappedComponent :type "PrimitiveComponent Object Reference") (OtherActor :type "Actor Object Reference") (OtherComp :type "PrimitiveComponent Object Reference") (OtherBodyIndex :type Integer) (bFromSweep :type Boolean) (SweepResult :type "HitResult Structure (by ref)"))
  (bind _astop_down_character (cast `/Game/TopDownBP/Blueprints/TopDownCharacter` OtherActor))
  (bind _astop_down_game_mode (cast `/Game/TopDownBP/Blueprints/TopDownGameMode` (`GameplayStatics.GetGameMode`)))
  (if (`/Game/TopDownBP/Blueprints/TopDownGameMode.Countdown Active` _astop_down_game_mode)
    (`self.EnableInput` (`GameplayStatics.GetPlayerController` (`/Game/TopDownBP/Blueprints/TopDownCharacter.Player Index` _astop_down_character)))
    (bind _hudref (`/Game/TopDownBP/Blueprints/TopDownCharacter.Hudref` _astop_down_character))
    (`/Game/Widget/HUD.Set Help Text` _hudref "Press E to Evacuate Station")
    (else
      (`/Game/Widget/HUD.Set Help Text` _hudref "Activate Security Console to Unlock Elevator"))))

(event `self.Box.OnComponentEndOverlap`
  (params (OverlappedComponent :type "PrimitiveComponent Object Reference") (OtherActor :type "Actor Object Reference") (OtherComp :type "PrimitiveComponent Object Reference") (OtherBodyIndex :type Integer))
  (bind _astop_down_character (cast `/Game/TopDownBP/Blueprints/TopDownCharacter` OtherActor))
  (`self.DisableInput` (`GameplayStatics.GetPlayerController` (`/Game/TopDownBP/Blueprints/TopDownCharacter.Player Index` _astop_down_character)))
  (`/Game/Widget/HUD.Set Help Text` (`/Game/TopDownBP/Blueprints/TopDownCharacter.Hudref` _astop_down_character) ""))

(event `InputAction|Interact`
  (params (Key :type "Key Structure"))
  (:`Pressed`
    (bind _ascurrent_game_settings (cast `/Game/CurrentGameSettings` (`GameplayStatics.GetGameInstance`)))
    (if (`/Game/CurrentGameSettings.Endless` _ascurrent_game_settings)
      (set `/Game/CurrentGameSettings.Level` (+ (`/Game/CurrentGameSettings.Level` _ascurrent_game_settings) 1) _ascurrent_game_settings)
      (bind _outactors (`GameplayStatics.GetAllActorsOfClass` "/Game/TopDownBP/Blueprints/TopDownCharacter.TopDownCharacter_C"))
      (for _array_element _outactors
        (`/Game/TopDownBP/Blueprints/TopDownCharacter.Save Data` _array_element (`/Game/TopDownBP/Blueprints/TopDownCharacter.Player Index` _array_element)))
      (`GameplayStatics.OpenLevel` "AlphaLayput")
      (else
        (`GameplayStatics.SetGamePaused` true)
        (bind _outactors_2 (`GameplayStatics.GetAllActorsOfClass` "/Game/TopDownBP/Blueprints/TopDownCharacter.TopDownCharacter_C"))
        (for _array_element_2 _outactors_2
          (`SceneComponent.SetVisibility` (`Character.CapsuleComponent` _array_element_2) false true)
          (`Widget.RemoveFromParent` (`/Game/TopDownBP/Blueprints/TopDownCharacter.Hudref` _array_element_2))
          (bind _returnvalue (`GameplayStatics.GetPlayerController` (`/Game/TopDownBP/Blueprints/TopDownCharacter.Player Index` _array_element_2)))
          (bind _returnvalue_2 (`|CreateWidget` "/Game/Widget/GameOver.GameOver_C" _returnvalue))
          (`/Game/Widget/GameOver.Player Escaped` _returnvalue_2 _array_element_2)
          (`UserWidget.AddToPlayerScreen` _returnvalue_2 0)
          (`WidgetBlueprintLibrary.SetInputMode_UIOnlyEx` _returnvalue _returnvalue_2))))))

(fn `UserConstructionScript`)