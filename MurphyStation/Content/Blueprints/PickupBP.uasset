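; Base pickup actor that scatters on spawn and can be collected by a TopDownCharacter.
; BeginPlay gives the mesh a random impulse, then after a delay a timeline fades a dynamic material's Alpha and destroys the actor.
; Box overlap calls PickUp with the character and destroys the actor on success; PickUp here only returns false, so any effect must come from an override.
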(event `self.ReceiveBeginPlay`
  (`PrimitiveComponent.AddImpulse` (`self.Static Mesh`) (`KismetMathLibrary.MakeVector` (`KismetMathLibrary.RandomFloatInRange` -200.0 200.0) (`KismetMathLibrary.RandomFloatInRange` -200.0 200.0) (`KismetMathLibrary.RandomFloatInRange` 0.0 300.0)) "None" false)
  (`KismetSystemLibrary.Delay` 10.0)
  (bind _returnvalue (`PrimitiveComponent.CreateDynamicMaterialInstance` (`self.Static Mesh`) 0 null "None"))
  (bind (_direction _alpha) (`Timeline|Fade Away` :!via `PlayFromStart`)
    (:`Update`
      (`MaterialInstanceDynamic.SetScalarParameterValue` _returnvalue "Alpha" _alpha))
    (:`Finished`
      (`self.K2_DestroyActor`))))

(event `self.Box Collision.OnComponentBeginOverlap`
  (params (OverlappedComponent :type "PrimitiveComponent Object Reference") (OtherActor :type "Actor Object Reference") (OtherComp :type "PrimitiveComponent Object Reference") (OtherBodyIndex :type Integer) (bFromSweep :type Boolean) (SweepResult :type "HitResult Structure (by ref)"))
  (bind _astop_down_character (cast `/Game/TopDownBP/Blueprints/TopDownCharacter` OtherActor))
  (bind _used (`self.Pick Up` _astop_down_character))
  (if _used
    (`self.K2_DestroyActor`)))

(fn `Pick Up`
  (params (Player :type "/Game/TopDownBP/Blueprints/TopDownCharacter Object Reference"))
  (returns (Used :type Boolean))
  (return false))

(fn `UserConstructionScript`)