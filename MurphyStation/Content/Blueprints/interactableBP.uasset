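; Base interactable actor that shows a help prompt when the TopDownCharacter enters its box trigger.
; Box overlap begin calls Show Text, which sets the HUD help text to DisplayText if CanInteract is true.
; Overlap end calls Hide Text to clear it.
; Interact is an empty function that takes the player.
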(event `self.Box.OnComponentBeginOverlap`
  (params (OverlappedComponent :type "PrimitiveComponent Object Reference") (OtherActor :type "Actor Object Reference") (OtherComp :type "PrimitiveComponent Object Reference") (OtherBodyIndex :type Integer) (bFromSweep :type Boolean) (SweepResult :type "HitResult Structure (by ref)"))
  (bind _astop_down_character (cast `/Game/TopDownBP/Blueprints/TopDownCharacter` OtherActor))
  (`self.Show Text` _astop_down_character))

(event `self.Box.OnComponentEndOverlap`
  (params (OverlappedComponent :type "PrimitiveComponent Object Reference") (OtherActor :type "Actor Object Reference") (OtherComp :type "PrimitiveComponent Object Reference") (OtherBodyIndex :type Integer))
  (bind _astop_down_character (cast `/Game/TopDownBP/Blueprints/TopDownCharacter` OtherActor))
  (`self.Hide Text` _astop_down_character))

(fn `Hide Text`
  (params (Player :type "/Game/TopDownBP/Blueprints/TopDownCharacter Object Reference"))
  (`/Game/Widget/HUD.Set Help Text` (`/Game/TopDownBP/Blueprints/TopDownCharacter.Hudref` Player) ""))

(fn `Interact`
  (params (Player :type "/Game/TopDownBP/Blueprints/TopDownCharacter Object Reference")))

(fn `Show Text`
  (params (Player :type "/Game/TopDownBP/Blueprints/TopDownCharacter Object Reference"))
  (if (`self.Can Interact`)
    (`/Game/Widget/HUD.Set Help Text` (`/Game/TopDownBP/Blueprints/TopDownCharacter.Hudref` Player) (`self.Display Text`))))

(fn `UserConstructionScript`)