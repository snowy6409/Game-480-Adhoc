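; DamageUpgrade is a pickup actor that raises weapon damage for the player who interacts with it.
; On Interact it increments the player's DamageModifier entry at the equipped weapon's WeaponType index, then destroys itself.
; An older method that added per-weapon UpgradeValues to BulletDamage remains in the graph but never runs.
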(event `/Game/Blueprints/interactableBP.Interact`
  (params (Player :type "/Game/TopDownBP/Blueprints/TopDownCharacter Object Reference"))
  (bind _damage_modifier (`/Game/TopDownBP/Blueprints/TopDownCharacter.Damage Modifier` Player))
  (bind _weapon_type (`/Game/Blueprints/Weapons/WeaponBP.Weapon Type` (`/Game/TopDownBP/Blueprints/TopDownCharacter.Equipped` Player)))
  (`KismetArrayLibrary.Array_Set` _damage_modifier _weapon_type (+ (`|GetArrayItem` _damage_modifier _weapon_type) 1))
  (`self.K2_DestroyActor`))

(fn `UserConstructionScript`
  (`parent.UserConstructionScript`))