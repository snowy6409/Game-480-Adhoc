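; A modular room actor that opens walls by direction flags, randomizes its lighting unless forced on, and manages enemy encounters.
; When the TopDownCharacter enters its sphere, it reveals child actors and, if allowed, spawns AIPawns or turrets at random navmesh points; leaving hides the children.
; Spawning re-arms after a delay with a count capped at half the maximum.
; SpawnLayout places a random layout in quarter-turn rotations, but is not called here.
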(event `self.ReceiveBeginPlay`
  (set `self.Spawn Count` (`KismetMathLibrary.RandomIntegerInRange` (`self.Min Enemies`) (`KismetMathLibrary.Clamp` (`self.Max Enemies`) (`self.Min Enemies`) 20)))
  (`self.Set Wall State`)
  (if (`self.Lights Always On`)
    (`self.Turn On Lights` :!label _label)
    (elif (`KismetMathLibrary.RandomBool`)
      (goto _label)
      (else
        (`self.Turn Off Lights`)))))

(event `self.Sphere.OnComponentBeginOverlap`
  (params (OverlappedComponent :type "PrimitiveComponent Object Reference") (OtherActor :type "Actor Object Reference") (OtherComp :type "PrimitiveComponent Object Reference") (OtherBodyIndex :type Integer) (bFromSweep :type Boolean) (SweepResult :type "HitResult Structure (by ref)"))
  (cast `/Game/TopDownBP/Blueprints/TopDownCharacter` OtherActor)
  (for _array_element (`self.GetAllChildActors` true)
    (`SceneComponent.SetVisibility` (`Actor.RootComponent` _array_element) true false)
    (if (`self.Can Spawn`)
      (`self.Spawn Enemies`))))

(event `self.Sphere.OnComponentEndOverlap`
  (params (OverlappedComponent :type "PrimitiveComponent Object Reference") (OtherActor :type "Actor Object Reference") (OtherComp :type "PrimitiveComponent Object Reference") (OtherBodyIndex :type Integer))
  (cast `/Game/TopDownBP/Blueprints/TopDownCharacter` OtherActor)
  (for _array_element (`self.GetAllChildActors` true)
    (`SceneComponent.SetVisibility` (`Actor.RootComponent` _array_element) false false)))

(event `Spawn Enemies`
  (bind _randomlocation (`NavigationSystemV1.K2_GetRandomLocationInNavigableRadius` (+ (`self.K2_GetActorLocation`) (0.0 0.0 20.0)) (`KismetMathLibrary.Conv_IntToDouble` (`self.Spawn Radius`)) null null))
  (for _ (range 1 (+ (`self.Spawn Count`) 1))
    (if (< (`KismetMathLibrary.RandomIntegerInRange` 0 2) 2)
      (`|SpawnActorFromClass` "/Game/Enemies/AIPawn.AIPawn_C" (`KismetMathLibrary.MakeTransform` (+ _randomlocation (0.0 0.0 200.0))) "AdjustIfPossibleButAlwaysSpawn" "OverrideRootScale" null null)
      (else
        (`|SpawnActorFromClass` "/Game/Enemies/TurretAI.TurretAI_C" (`KismetMathLibrary.MakeTransform` _randomlocation) "AdjustIfPossibleButAlwaysSpawn" "OverrideRootScale" null null))))
  (set `self.Can Spawn` false)
  (`self.Reset Spawn`))

(event `Reset Spawn`
  (`KismetSystemLibrary.Delay` (`KismetMathLibrary.Conv_IntToDouble` (`self.Respawn Delay`)))
  (set `self.Spawn Count` (`KismetMathLibrary.RandomIntegerInRange` 1 (/ (`self.Max Enemies`) 2)))
  (set `self.Can Spawn` true))

(fn `Set Wall State`
  (bind _leftw (`self.LeftW`))
  (bind _downw (`self.DownW`))
  (bind _rightw (`self.RightW`))
  (bind _upw (`self.UpW`))
  (if (`self.Up`)
    (`SceneComponent.SetVisibility` _upw false false)
    (`PrimitiveComponent.SetCollisionEnabled` _upw "NoCollision"))
  (if (`self.Down`)
    (`SceneComponent.SetVisibility` _downw false false)
    (`PrimitiveComponent.SetCollisionEnabled` _downw "NoCollision"))
  (if (`self.Left`)
    (`SceneComponent.SetVisibility` _leftw false false)
    (`PrimitiveComponent.SetCollisionEnabled` _leftw "NoCollision"))
  (if (`self.Right`)
    (`SceneComponent.SetVisibility` _rightw false false)
    (`PrimitiveComponent.SetCollisionEnabled` _rightw "NoCollision")))

(fn `Spawn Layout`
  (params (`Possible Layouts` :type "Array of /Game/Rooms/RoomLayoutBP Class Reference"))
  (`|SpawnActorFromClass` (`|GetArrayItem` `Possible Layouts` (`KismetMathLibrary.RandomIntegerInRange` 0 (`KismetArrayLibrary.Array_LastIndex` `Possible Layouts`))) (`KismetMathLibrary.MakeTransform` (+ (`self.K2_GetActorLocation`) (0.0 0.0 15.0)) (`KismetMathLibrary.MakeRotator` 0.0 0.0 (* (`KismetMathLibrary.RandomIntegerInRange` 0 3) 90.0))) "AlwaysSpawn" "OverrideRootScale" null null))

(fn `Turn Off Lights`
  (for _array_element (`self.GetAllChildActors` true)
    (bind _aslight_bp (cast `/Game/Blueprints/LightBP` _array_element))
    (`/Game/Blueprints/LightBP.TurnOff` _aslight_bp)))

(fn `Turn On Lights`
  (for _array_element (`self.GetAllChildActors` true)
    (bind _aslight_bp (cast `/Game/Blueprints/LightBP` _array_element))
    (`/Game/Blueprints/WallLight.TurnOn` _aslight_bp)))

(fn `UserConstructionScript`)