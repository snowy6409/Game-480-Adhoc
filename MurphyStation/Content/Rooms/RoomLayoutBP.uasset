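; Room layout Blueprint that randomly populates marker components with containers and recovery stations.
; SpawnContainer usually leaves the spot empty, otherwise placing a Locker or, more rarely, a WeaponCrate through a nested roll.
; SpawnRecoveryStation gives equal odds to a HealthStation or OxygenStation, and spawns nothing half the time.
; Both functions spawn at the passed component's world transform and then destroy that component, whatever the outcome.
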(fn `Spawn Container`
  (params (Target :type "ArrowComponent Object Reference"))
  (bind _returnvalue (`SceneComponent.K2_GetComponentToWorld` Target))
  (if (== (`KismetMathLibrary.RandomIntegerInRange` 0 4) 0)
    (if (== (`KismetMathLibrary.RandomIntegerInRange` 0 4) 0)
      (`|SpawnActorFromClass` "/Game/Blueprints/WeaponCrate.WeaponCrate_C" _returnvalue "AlwaysSpawn" "OverrideRootScale" null null)
      (else
        (`|SpawnActorFromClass` "/Game/Blueprints/Locker.Locker_C" _returnvalue "AlwaysSpawn" "OverrideRootScale" null null))))
  (`ActorComponent.K2_DestroyComponent` Target))

(fn `Spawn Recovery Station`
  (params (Target :type "ArrowComponent Object Reference"))
  (bind _returnvalue (`SceneComponent.K2_GetComponentToWorld` Target))
  (switch `int` (`KismetMathLibrary.RandomIntegerInRange` 0 3)
    (:`Default`
      _)
    (:`0`
      (`|SpawnActorFromClass` "/Game/Blueprints/HealthStation.HealthStation_C" _returnvalue "Undefined" "OverrideRootScale" null null))
    (:`1`
      (`|SpawnActorFromClass` "/Game/Blueprints/OxygenStation.OxygenStation_C" _returnvalue "Undefined" "OverrideRootScale" null null))
    (:`2`
      _)
    (:`3`
      _))
  (`ActorComponent.K2_DestroyComponent` Target))

(fn `UserConstructionScript`)