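; Large room Blueprint, a child room class that can spawn a boss or a self-destruct console.
; SpawnEnemies runs the parent logic, then calls SpawnBoss, which places the boss above the room origin once, only when the room is flagged as a boss room.
; SpawnConsole places a SelfDestructConsole at the room's location, though nothing in this Blueprint calls it.
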(event `self.Spawn Enemies`
  (`parent.Spawn Enemies`)
  (`self.Spawn Boss`))

(fn `Spawn Boss`
  (if (and (`self.Boss Room`) (not (`self.Boss Spawned`)))
    (`|SpawnActorFromClass` "/Game/Enemys/Boss.Boss_C" (`KismetMathLibrary.MakeTransform` (+ (`self.K2_GetActorLocation`) (0.0 0.0 400.0))) "AdjustIfPossibleButAlwaysSpawn" "OverrideRootScale" null null)
    (set `self.Boss Spawned` true)))

(fn `Spawn Console`
  (`|SpawnActorFromClass` "/Game/Blueprints/SelfDestructConsole.SelfDestructConsole_C" (`KismetMathLibrary.MakeTransform` (`self.K2_GetActorLocation`)) "Undefined" "OverrideRootScale" null null))

(fn `UserConstructionScript`
  (`parent.UserConstructionScript`))