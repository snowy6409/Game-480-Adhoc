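; Weapon Blueprint that fires damage-carrying projectiles for a player and initializes its ammo to the magazine size on BeginPlay.
; Fire spawns a FirstPersonProjectile at the given transform, passing it the player and base damage plus a scaled modifier.
; It then plays the fire sound at the weapon's location, scaled by master volume from the CurrentGameSettings game instance.
; Fire neither checks nor decrements ammo.
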(event `self.ReceiveBeginPlay`
  (set `self.Current Ammo` (`self.Magazine Size`)))

(fn `Fire`
  (params (`Bullet Transform` :type "Transform Structure") (`Damage Modifier` :type Integer) (Player :type "/Game/TopDownBP/Blueprints/TopDownCharacter Object Reference"))
  (bind _returnvalue (`|SpawnActorFromClass` "/Game/FirstPersonBP/Blueprints/FirstPersonProjectile.FirstPersonProjectile_C" `Bullet Transform` "Undefined" "OverrideRootScale" null null))
  (set `/Game/FirstPersonBP/Blueprints/FirstPersonProjectile.Player` Player _returnvalue)
  (set `/Game/FirstPersonBP/Blueprints/FirstPersonProjectile.Damage` (+ (`self.Base Damage`) (* `Damage Modifier` (`self.Damage Scaling`))) _returnvalue)
  (bind _ascurrent_game_settings (cast `/Game/CurrentGameSettings` (`GameplayStatics.GetGameInstance`)))
  (`GameplayStatics.PlaySoundAtLocation` (`self.Fire Sound`) (`self.K2_GetActorLocation`) (struct) (`/Game/CurrentGameSettings.MasterVolume` _ascurrent_game_settings) 1.0 0.0 null null null))

(fn `UserConstructionScript`)